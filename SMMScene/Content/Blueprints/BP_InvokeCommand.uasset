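; Command-pattern invoker actor that runs place commands and manages their undo and redo history.
; InvokeCommandPlace spawns a BP_PlaceCommand actor at the origin, calls Place and pushes it onto UndoStack.
; UndoLast and RedoLast call UndoMessage or RedoMessage on the newest entry and move it to the opposite stack.
; New placements leave RedoStack intact, and the CommandPlace reference cached at BeginPlay is unused in these graphs.
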(event `self.ReceiveBeginPlay`
  (bind _returnvalue (`GameplayStatics.GetActorOfClass` "/Game/Blueprints/BP_PlaceCommand.BP_PlaceCommand_C"))
  (set `self.CommandPlace` _returnvalue))

(fn `InvokeCommandPlace`
  (bind _returnvalue (`|SpawnActorFromClass` "/Game/Blueprints/BP_PlaceCommand.BP_PlaceCommand_C" (`KismetMathLibrary.MakeTransform` (0.0 0.0 0.0)) "Undefined" "MultiplyWithRoot" null null))
  (`/Engine/EditorBlueprintResources/StandardMacros.IsValid` _returnvalue
    (:`Is Valid`
      (`/Game/Blueprints/BPI_Command.Place` _returnvalue)
      (`KismetArrayLibrary.Array_Add` (`self.UndoStack`) _returnvalue))))

(fn `RedoLast`
  (bind _redostack (`self.RedoStack`))
  (bind _returnvalue (+ (`KismetArrayLibrary.Array_Length` _redostack) -1))
  (bind _output (`|GetArrayItem` _redostack _returnvalue))
  (`/Engine/EditorBlueprintResources/StandardMacros.IsValid` _output
    (:`Is Valid`
      (message `/Game/Blueprints/BPI_Command.Redo` _output)
      (`KismetArrayLibrary.Array_Add` (`self.UndoStack`) _output)
      (`KismetArrayLibrary.Array_Remove` (`self.RedoStack`) _returnvalue))))

(fn `UndoLast`
  (bind _returnvalue (+ (`KismetArrayLibrary.Array_Length` (`self.UndoStack`)) -1))
  (bind _output (`|GetArrayItem` (`self.UndoStack`) _returnvalue))
  (if (`KismetArrayLibrary.Array_IsValidIndex` (`self.UndoStack`) _returnvalue)
    (message `/Game/Blueprints/BPI_Command.Undo` _output)
    (`KismetArrayLibrary.Array_Add` (`self.RedoStack`) _output)
    (`KismetArrayLibrary.Array_Remove` (`self.UndoStack`) _returnvalue)))

(fn `UserConstructionScript`)