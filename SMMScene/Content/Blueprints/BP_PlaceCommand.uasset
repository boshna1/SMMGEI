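; BP_PlaceCommand is a command object for placing objects in the world, with Place, Undo and Redo events.
; On BeginPlay it caches the player character as BP_Player.
; Place spawns the player's Target class at RayEnd if CanPlace is true, storing the transform and spawned actor.
; Undo destroys that actor; Redo respawns the player's current Target at the stored transform, again gated by CanPlace.
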(event `self.ReceiveBeginPlay`
  (bind _asbp_player (cast `/Game/Blueprints/BP_Player` (`GameplayStatics.GetPlayerCharacter` 0)))
  (set `self.PlayerRef` _asbp_player))

(event `/Game/Blueprints/BPI_Command.Place`
  (bind _playerref (`self.PlayerRef`))
  (bind _returnvalue (`KismetMathLibrary.Conv_VectorToTransform` (`/Game/Blueprints/BP_Player.RayEnd` _playerref)))
  (if (`/Game/Blueprints/BP_Player.CanPlace` _playerref)
    (bind _returnvalue_2 (`|SpawnActorFromClass` (`/Game/Blueprints/BP_Player.Target` _playerref) _returnvalue "Undefined" "MultiplyWithRoot" null null))
    (set `self.POTransform` _returnvalue)
    (set `self.PlacedObject` _returnvalue_2)))

(event `/Game/Blueprints/BPI_Command.Undo`
  (bind _placedobject (`self.PlacedObject`))
  (`/Engine/EditorBlueprintResources/StandardMacros.IsValid` _placedobject
    (:`Is Valid`
      (`self.K2_DestroyActor` _placedobject))))

(event `/Game/Blueprints/BPI_Command.Redo`
  (bind _playerref (`self.PlayerRef`))
  (bind _potransform (`self.POTransform`))
  (if (`/Game/Blueprints/BP_Player.CanPlace` _playerref)
    (bind _returnvalue (`|SpawnActorFromClass` (`/Game/Blueprints/BP_Player.Target` _playerref) _potransform "Undefined" "MultiplyWithRoot" null null))
    (set `self.PlacedObject` _returnvalue)
    (set `self.POTransform` _potransform)))

(fn `UserConstructionScript`)