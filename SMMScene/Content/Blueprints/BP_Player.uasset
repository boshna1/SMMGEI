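; Player pawn for placing primitive shapes (sphere, cube, cylinder, cone) with undo and redo through a command invoker.
; Enhanced Input drives movement along the right and up vectors, selects the Target shape, and forwards place, undo and redo to the level's BP_InvokeCommand.
; Tick draws a forward debug trace and stores its end point in RayEnd, ignoring the hit result.
; The placement cooldown logic is disconnected.
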(event `self.ReceiveBeginPlay`
  (bind _asplayer_controller (cast `PlayerController` (`GameplayStatics.GetPlayerController` 0)))
  (bind _returnvalue (pcsubsystem `EnhancedInputLocalPlayerSubsystem` _asplayer_controller))
  (`/Engine/EditorBlueprintResources/StandardMacros.IsValid` _returnvalue
    (:`Is Valid`
      (`EnhancedInputSubsystemInterface.AddMappingContext` _returnvalue "/Game/Blueprints/Actions/IMC_Player.IMC_Player" 0 (struct))
      (set `self.RayDistance` 300.0)
      (set `self.CanPlace` true)
      (bind _returnvalue_2 (`GameplayStatics.GetActorOfClass` "/Game/Blueprints/BP_InvokeCommand.BP_InvokeCommand_C"))
      (set `self.CommandInvoker` _returnvalue_2))))

(event `EnhancedInput|/Game/Blueprints/Actions/IA_Move`
  (params (ActionValue :type "Vector2D Structure") (ElapsedSeconds :type "Float (double-precision)") (TriggeredSeconds :type "Float (double-precision)") (InputAction :type "InputAction Object Reference" :default "/Game/Blueprints/Actions/IA_Move.IA_Move"))
  (bind (_x _y) (`KismetMathLibrary.BreakVector2D` ActionValue))
  (:`Triggered`
    (`self.AddMovementInput` (`self.GetActorRightVector`) _x)
    (`self.AddMovementInput` (`self.GetActorUpVector`) _y)))

(event `self.ReceiveTick`
  (params (DeltaSeconds :type "Float (single-precision)"))
  (bind _location (.location (`self.GetTransform`)))
  (bind _returnvalue (+ _location (* (`self.GetActorForwardVector`) (`self.RayDistance`))))
  (bind _outhit (`KismetSystemLibrary.LineTraceSingle` :`Start` _location :`End` _returnvalue :`TraceChannel` "TraceTypeQuery1" :`DrawDebugType` "ForOneFrame"))
  (set `self.RayEnd` _returnvalue))

(event `CanPlaceCooldown`
  (set `self.CanPlace` true))

(event `EnhancedInput|/Game/Blueprints/Actions/IA_Place`
  (params (ActionValue :type Boolean) (ElapsedSeconds :type "Float (double-precision)") (TriggeredSeconds :type "Float (double-precision)") (InputAction :type "InputAction Object Reference" :default "/Game/Blueprints/Actions/IA_Place.IA_Place"))
  (bind _commandinvoker (`self.CommandInvoker`))
  (:`Triggered`
    (`/Engine/EditorBlueprintResources/StandardMacros.IsValid` _commandinvoker
      (:`Is Valid`
        (`/Game/Blueprints/BP_InvokeCommand.InvokeCommandPlace` _commandinvoker)))))

(event `EnhancedInput|/Game/Blueprints/Actions/IA_Redo`
  (params (ActionValue :type Boolean) (ElapsedSeconds :type "Float (double-precision)") (TriggeredSeconds :type "Float (double-precision)") (InputAction :type "InputAction Object Reference" :default "/Game/Blueprints/Actions/IA_Redo.IA_Redo"))
  (bind _commandinvoker (`self.CommandInvoker`))
  (:`Triggered`
    (`/Engine/EditorBlueprintResources/StandardMacros.IsValid` _commandinvoker
      (:`Is Valid`
        (`/Game/Blueprints/BP_InvokeCommand.Redo` _commandinvoker)))))

(event `EnhancedInput|/Game/Blueprints/Actions/IA_Undo`
  (params (ActionValue :type Boolean) (ElapsedSeconds :type "Float (double-precision)") (TriggeredSeconds :type "Float (double-precision)") (InputAction :type "InputAction Object Reference" :default "/Game/Blueprints/Actions/IA_Undo.IA_Undo"))
  (bind _commandinvoker (`self.CommandInvoker`))
  (:`Triggered`
    (`/Engine/EditorBlueprintResources/StandardMacros.IsValid` _commandinvoker
      (:`Is Valid`
        (`/Game/Blueprints/BP_InvokeCommand.UndoLast` _commandinvoker)))))

(event `EnhancedInput|/Game/Blueprints/Actions/IA_Select`
  (params (ActionValue :type "Float (double-precision)") (ElapsedSeconds :type "Float (double-precision)") (TriggeredSeconds :type "Float (double-precision)") (InputAction :type "InputAction Object Reference" :default "/Game/Blueprints/Actions/IA_Select.IA_Select"))
  (:`Triggered`
    (switch `int` (`KismetMathLibrary.FTrunc` ActionValue)
      (:`1`
        (set `self.Target` "/Game/Blueprints/BP_Sphere.BP_Sphere_C"))
      (:`2`
        (set `self.Target` "/Game/Blueprints/BP_Cube.BP_Cube_C"))
      (:`3`
        (set `self.Target` "/Game/Blueprints/BP_Cylinder.BP_Cylinder_C"))
      (:`4`
        (set `self.Target` "/Game/Blueprints/BP_Cone.BP_Cone_C")))))

(fn `UserConstructionScript`)